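; Global FPS game mode that provides functions to initialize a match and spawn player characters.
; InitializeGame records the current level name and caches every PlayerStart transform.
; CreateNewCharacter gives a PlayerController_Global an incrementing player index, then SpawnCharacter spawns and possesses a Character_Global on authority, always at the first cached start, and copies the index onto it.
; The event graph is empty, so these functions rely on external callers.
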(event EventBeginPlay)

(event EventTick
  (params (DeltaSeconds :type Float%20%28single-precision%29)))

(fn ConstructionScript)

(fn CreatePlayerStartArray
  (bind _outactors (Actor|GetAllActorsOfClass "/Script/Engine.PlayerStart"))
  (for _array_element _outactors
    (Utilities|Array|Add (Variables|CurrentState|GetCharacterStart) (Transformation|GetActorTransform _array_element))))

(fn InitializeMap
  (bind _returnvalue (Game|GetCurrentLevelName true))
  (Variables|CurrentState|SetLevelPlaying _returnvalue))

(fn InitializeGame
  (CallFunction|InitializeMap)
  (CallFunction|CreatePlayerStartArray))

(fn CreateNewPlayerIndex
  (bind _output_get (Variables|CurrentState|SetPlayerCountNum (+ (Variables|CurrentState|GetPlayerCountNum) 1)))
  (return (- _output_get 1)))

(fn SpawnCharacter
  (params (InputIndex :type Integer) (InputController :type Player%20Controller%20Object%20Reference))
  (LocalVariables|SetLocalInputIndex InputIndex)
  (bind _output_get (LocalVariables|SetLocalInputController InputController))
  (Utilities|IsValid _output_get
    (:Is%20Valid
      (Networking|SwitchHasAuthority
        (:Authority
          (bind _returnvalue (Game|SpawnActorfromClass "/Game/Blueprint/Character_Global.Character_Global_C" (Utilities|Array|Get(acopy) (Variables|CurrentState|GetCharacterStart)) "Undefined" (LocalVariables|GetLocalInputController) 0))
          (bind _output_get_2 (LocalVariables|SetLocalSpawnResult _returnvalue))
          (Utilities|IsValid _output_get_2
            (:Is%20Valid
              (Pawn|Possess (LocalVariables|GetLocalInputController) (LocalVariables|GetLocalSpawnResult))
              (bind _output_get_3 (Variables|/Game/Blueprint/Character_Global.Character_Global_C|SetMyIndex (LocalVariables|GetLocalSpawnResult) (LocalVariables|GetLocalInputIndex)))
              (Utilities|Array|Add (Variables|/Game/Blueprint/Character_Global.Character_Global_C|GetViewIndex (LocalVariables|GetLocalSpawnResult)) _output_get_3)
              (return (LocalVariables|GetLocalSpawnResult)))))))))

(fn CreateNewCharacter
  (params (InputController :type Player%20Controller%20Object%20Reference))
  (bind _output_get (LocalVariables|SetTheController InputController))
  (Utilities|IsValid _output_get
    (:Is%20Valid
      (bind _asplayer_controller_global (Utilities|Casting|CastToPlayerController_Global (LocalVariables|GetTheController)))
      (bind _playerindex (CallFunction|CreateNewPlayerIndex))
      (bind _output_get_2 (Variables|/Game/Blueprint/PlayerController_Global.PlayerController_Global_C|SetPlayerIndex _asplayer_controller_global _playerindex))
      (bind _outputcharacter (CallFunction|SpawnCharacter _output_get_2 (LocalVariables|GetTheController)))
      (return _outputcharacter))))